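; Player controller that manages a toggleable HUD menu and respawns the player in a random vehicle.
; On BeginPlay it creates the hidden widget and starts a looping timer that shows it whenever the pawn is missing or a spectator.
; Reset inputs call a server event that replaces the pawn with a plane or car, weighted toward Sedan, at randomly picked PlayerStart transforms, then snap the chase camera after a delay.
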(event `self.ReceiveEndPlay`
  (params (EndPlayReason :type "EngineTypes.EEndPlayReason Enum" :default "ActorDestroyed"))
  (`Widget.RemoveFromParent` (`self.widgetHUD`)))

(event `self.ReceiveBeginPlay`
  (`|ExecutionSequence`
    (:`then_0`
      (`KismetSystemLibrary.K2_SetTimer` null "HUDIFDEAD" 0.33 true))
    (:`then_1`
      (`/Engine/EditorBlueprintResources/StandardMacros.IsValid` (`self.GetHUD`)
        (:`Is Valid`
          (bind _returnvalue (`|CreateWidget` "/Game/Blueprints/MyUMGHUD.MyUMGHUD_C" self))
          (add `/Game/Blueprints/MyUMGHUD.ClosePLZ` _returnvalue (delegate `CloseESC`))
          (`Widget.SetVisibility` _returnvalue "Collapsed")
          (set `self.widgetHUD` _returnvalue)
          (`UserWidget.AddToViewport` _returnvalue))))))

(event `HUDIFDEAD`
  (bind _returnvalue (`self.K2_GetPawn`))
  (`|ExecutionSequence`
    (:`then_0`
      (`/Engine/EditorBlueprintResources/StandardMacros.IsValid` _returnvalue
        (:`Is Not Valid`
          _)))
    (:`then_1`
      (cast `SpectatorPawn` _returnvalue)))
  (`Widget.SetVisibility` (`self.widgetHUD`) "Visible"))

(event `CloseESC`
  (`Widget.SetVisibility` (`self.widgetHUD`) "Collapsed"))

(event `Key|Gamepad_Special_Right`
  (:`Released`
    (`self.ResetCar_Server` (`KismetMathLibrary.RandomIntegerInRange` 0 10) :!label _label)
    (`KismetSystemLibrary.Delay` 1.0)
    (bind _outactors (`GameplayStatics.GetAllActorsOfClass` "/Game/Blueprints/CameraChase.CameraChase_C"))
    (`/Game/Blueprints/CameraChase.SnapCamera` (`KismetArrayLibrary.Array_Get` _outactors))))

(event `Key|Gamepad_Special_Left`
  (:`Released`
    (goto _label)))

(event `Key|Escape`
  (bind _widgethud (`self.widgetHUD`))
  (:`Released`
    (if (`Widget.IsVisible` _widgethud) :!label _label_2
      (`Widget.SetVisibility` _widgethud "Collapsed")
      (else
        (`Widget.SetVisibility` _widgethud "Visible")))))

(event `InputAction|ResetCar`
  (:`Pressed`
    (goto _label)))

(event `Key|Insert`
  (:`Released`
    (goto _label_2)))

(event `ResetCar_Server`
  (params (CarType :type Integer))
  (bind _returnvalue (`KismetMathLibrary.MakeTransform` (0.0 0.0 0.0)))
  (bind _returnvalue_2 (`self.K2_GetPawn`))
  (`|ExecutionSequence`
    (:`then_0`
      (`self.K2_DestroyActor` (`self.K2_GetPawn`))
      (switch `int` CarType
        (:`Default`
          (bind _returnvalue_3 (`|SpawnActorFromClass` "/Game/Sedan/Sedan.Sedan_C" _returnvalue :!label _label_3))
          (`self.Possess` self _returnvalue_3))
        (:`0`
          (bind _returnvalue_4 (`|SpawnActorFromClass` "/Game/Blueprints/BP_Plane.BP_Plane_C" _returnvalue))
          (`self.Possess` _returnvalue_4))
        (:`1`
          (bind _returnvalue_5 (`|SpawnActorFromClass` "/Game/Vehicle/VehicleBlueprint.VehicleBlueprint_C" _returnvalue))
          (`self.Possess` self _returnvalue_5))
        (:`2`
          (goto _label_3))))
    (:`then_1`
      (bind _outactors (`GameplayStatics.GetAllActorsOfClass` "/Script/Engine.PlayerStart"))
      (bind _item (`KismetArrayLibrary.Array_Get` _outactors (`KismetMathLibrary.RandomIntegerInRange` 0 (- (`KismetArrayLibrary.Array_Length` _outactors) 1))))
      (`self.K2_SetActorLocation` _returnvalue_2 (`self.K2_GetActorLocation` _item) false)
      (`self.SetActorRotation` _returnvalue_2 (`self.K2_GetActorRotation` _item)))))

(fn `UserConstructionScript`)