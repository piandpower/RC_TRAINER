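; CameraChase is a camera actor that follows whichever pawn the first player controls and can become that player's view.
; After a startup delay, a looping timer repeatedly moves it to the pawn's location and rotation and attaches it, so it relinks when the pawn changes.
; F1 release, left shoulder press or SnapCamera blends the view to it with a cubic blend.
; Disconnected offset and rotation nodes never run.
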(event `RelinkCamera`
  (bind _returnvalue (`Controller.K2_GetPawn` (`GameplayStatics.GetPlayerController` 0)))
  (`/Engine/EditorBlueprintResources/StandardMacros.IsValid` (`GameplayStatics.GetPlayerPawn` 0)
    (:`Is Valid`
      (`self.K2_SetActorLocation` (`self.K2_GetActorLocation` _returnvalue))
      (`self.SetActorRotation` (`self.K2_GetActorRotation` _returnvalue))
      (`self.K2_AttachRootComponentToActor` self _returnvalue "None" "KeepWorldPosition" true))))

(event `self.ReceiveBeginPlay`
  (`KismetSystemLibrary.Delay` 1.0)
  (`KismetSystemLibrary.K2_SetTimer` null "RelinkCamera" 1.0 true))

(event `SnapCamera`
  (`PlayerController.SetViewTargetWithBlend` (`GameplayStatics.GetPlayerController` 0) self 1.0 "VTBlend_Cubic" 0.0 false :!label _label))

(event `Key|F1`
  (:`Released`
    (goto _label)))

(event `Key|Gamepad_LeftShoulder`
  (:`Pressed`
    (goto _label)))

(event `self.ReceiveTick`
  (params (DeltaSeconds :type "Float (single-precision)")))

(fn `UserConstructionScript`)