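; CameraPerson is a movable camera actor that keeps its view aimed at the first player's pawn.
; Each Tick it slides along world X and Y from gamepad D-pad input and rotates Camera1 with a look-at rotation toward the pawn.
; SnapCamera blends the player controller's view to this actor, triggered shortly after BeginPlay, by the right shoulder button, or on F2 release.
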(event `self.ReceiveTick`
  (params (DeltaSeconds :type "Float (single-precision)"))
  (`/Engine/EditorBlueprintResources/StandardMacros.IsValid` (`GameplayStatics.GetPlayerPawn` 0)
    (:`Is Valid`
      (`|ExecutionSequence`
        (:`then_0`
          (if (or (!= (`self.moveY`) 0.0) (!= (`self.moveX`) 0.0))
            (`SceneComponent.K2_SetWorldLocation` self (`KismetMathLibrary.MakeVector` (+ (.x (`SceneComponent.K2_GetComponentLocation` self)) (* (`self.moveX`) DeltaSeconds 1000.0)) (+ (.y (`SceneComponent.K2_GetComponentLocation` self)) (* (`self.moveY`) DeltaSeconds 1000.0)) (.z (`SceneComponent.K2_GetComponentLocation` self))) false)))
        (:`then_1`
          (`SceneComponent.K2_SetWorldRotation` (`self.Camera1`) (`KismetMathLibrary.FindLookAtRotation` (`SceneComponent.K2_GetComponentLocation` (`self.Camera1`)) (`self.K2_GetActorLocation` (`GameplayStatics.GetPlayerPawn` 0))) false))))))

(event `Key|Gamepad_DPad_Right`
  (:`Pressed`
    (set `self.moveY` 1.0))
  (:`Released`
    (set `self.moveY` 0.0)))

(event `Key|Gamepad_DPad_Up`
  (:`Pressed`
    (set `self.moveX` 1.0))
  (:`Released`
    (set `self.moveX` 0.0)))

(event `Key|Gamepad_DPad_Left`
  (:`Pressed`
    (set `self.moveY` -1.0))
  (:`Released`
    (set `self.moveY` 0.0)))

(event `Key|Gamepad_DPad_Down`
  (:`Pressed`
    (set `self.moveX` -1.0))
  (:`Released`
    (set `self.moveX` 0.0)))

(event `SnapCamera`
  (`PlayerController.SetViewTargetWithBlend` (`GameplayStatics.GetPlayerController` 0) self 1.0 "VTBlend_Linear" 0.0 false :!label _label))

(event `Key|Gamepad_RightShoulder`
  (:`Pressed`
    (goto _label)))

(event `Key|F2`
  (:`Released`
    (goto _label)))

(event `self.ReceiveBeginPlay`
  (`KismetSystemLibrary.Delay` 1.0)
  (goto _label))

(fn `UserConstructionScript`)